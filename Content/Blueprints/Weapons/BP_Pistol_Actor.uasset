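; Pistol weapon actor, a child Blueprint that supplies the pistol's own firing animation and sound.
; FireEvent plays the pistol fire montage on the owning character's mesh, then immediately plays the fire sound at the weapon's Barrel_Socket.
; The parent FireEvent call is unwired, so inherited fire logic does not run, and no damage or projectile logic appears here.
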(event EventBeginPlay
  (|CallParentFunction) ; This node is disabled and will not be called.\nDrag off pins to build functionality.
)

(event Collision|EventActorBeginOverlap
  (params (OtherActor :type Actor%20Object%20Reference))
  (|CallParentFunction OtherActor) ; This node is disabled and will not be called.\nDrag off pins to build functionality.
)

(event EventTick
  (params (DeltaSeconds :type Float%20%28single-precision%29))
  (|CallParentFunction DeltaSeconds) ; This node is disabled and will not be called.\nDrag off pins to build functionality.
)

(event EventFireEvent
  (bind _skeletalmesh (Variables|Default|GetSkeletalMesh))
  (Animation|Montage|PlayMontage (Variables|/Script/Engine.Character|GetMesh (Variables|Default|GetCharacterOwner)) "/Game/Assets/Characters/Simple/Animations/Pistol/MM_Pistol_Fire_Montage.MM_Pistol_Fire_Montage"
    (:then
      (Audio|PlaySoundatLocation "/Game/Blueprints/sound/SC_Pitol_Fire.SC_Pitol_Fire" (Transformation|GetSocketLocation _skeletalmesh "Barrel_Socket") (Transformation|GetSocketRotation _skeletalmesh "Barrel_Socket") 1.0 1.0 0.0 0 0 0 0))))

(fn ConstructionScript
  (|CallParentFunction))